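; Enemy-side core actor that acts as a hit-point objective for enemy1 units to reach.
; When an enemy1 overlaps its capsule, the core destroys that enemy and loses one CoreHP.
; It prints an under-attack message, or "Game Over" once HP reaches zero, with no further end-game logic.
; The construction script tags the actor as "core".
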(event `self.Capsule.OnComponentBeginOverlap`
  (params (OverlappedComponent :type "PrimitiveComponent Object Reference") (OtherActor :type "Actor Object Reference") (OtherComp :type "PrimitiveComponent Object Reference") (OtherBodyIndex :type Integer) (bFromSweep :type Boolean) (SweepResult :type "HitResult Structure (by ref)"))
  (bind _asenemy_1 (cast `/Game/TriggerForCommander/blueprints/enemy/ThirdPersonBP/Blueprints/enemy1` OtherActor))
  (`self.K2_DestroyActor` _asenemy_1)
  (set `self.Core_HP` (- (`self.Core_HP`) 1))
  (if (<= (`self.Core_HP`) 0)
    (`KismetSystemLibrary.PrintString` "Game Over")
    (else
      (`KismetSystemLibrary.PrintString` "Core is under attack!"))))

(fn `UserConstructionScript`
  (set `self.Tags` (`|MakeArray` "core" :!type "Name")))