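; Wave spawner actor that runs timed enemy waves and pays the player gold when each one ends.
; Tick counts down to each wave, then spawns Enemy1 AI at SpawnPoint on a fixed delay while the wave runs.
; Spawned enemies join EnemyList with a back-reference to the spawner; an empty list ends the wave.
; The per-wave Enemies count grows with the wave number but does not limit spawning here.
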(event `self.ReceiveBeginPlay`
  ;[1 1 1] Begin Play Event - Find Player
  (bind _outactors (`GameplayStatics.GetAllActorsOfClassWithTag` "/Game/FirstPersonCPP/Blueprints/FirstPersonCharacter.FirstPersonCharacter_C" "Player"))
  (bind _asfirst_person_character (cast `/Game/FirstPersonCPP/Blueprints/FirstPersonCharacter` (`|GetArrayItem` _outactors))
    (:`then`
      (set `self.Player` _asfirst_person_character)
      (`KismetSystemLibrary.PrintString` "Hello"))
    (:`CastFailed`
      (`KismetSystemLibrary.PrintString` "Error!"))))

(event `self.ReceiveTick`
  (params (DeltaSeconds :type "Float (single-precision)"))
  (bind _wavetimer (`self.WaveTimer`))
  ;[1 1 1] Check Wave End
  (if (`self.WaveStart`)
    (if (== (`KismetArrayLibrary.Array_Length` (`self.EnemyList`)) 0)
      (`self.EndWave`)))
  ;[1 1 1] Check Start Wave
  (if (<= _wavetimer 0.0)
    (set `self.WaveTimer` 0.0)
    (else
      (bind _output_get (set `self.WaveTimer` (- _wavetimer DeltaSeconds)))
      (if (<= _output_get 0.0)
        (if (not (`self.WaveStart`))
          (`self.StartWave`)))))
  ;[1 1 1] Check Enemy Spawn Time
  (bind _output_get_2 (set `self.SpawnDelay` (- (`self.SpawnDelay`) DeltaSeconds)))
  (if (<= _output_get_2 0.0)
    (if (`self.WaveStart`)
      (`self.SpawnEnemy`)
      (set `self.SpawnDelay` 3.0))))

(event `StartWave`
  (bind _wave (`self.Wave`))
  ;[1 1 1] Wave Start - Set Wave Number / Set Enemy Quantity
  (set `self.Wave` (+ _wave 1))
  (set `self.Enemies` (+ _wave 4))
  (set `self.WaveStart` true)
  (`KismetSystemLibrary.PrintString` "Wave Start"))

(event `EndWave`
  (bind _player (`self.Player`))
  ;[1 1 1] Wave End - Set Next Wave Timer / Give Gold to Player
  (set `self.WaveStart` false)
  (set `self.WaveTimer` 30.0)
  (set `/Game/FirstPersonCPP/Blueprints/FirstPersonCharacter.Gold` (+ (`/Game/FirstPersonCPP/Blueprints/FirstPersonCharacter.Gold` _player) 100) _player))

(event `SpawnEnemy`
  ;[1 1 1] Spawn Enemy Event
  (bind _returnvalue (`AIBlueprintHelperLibrary.SpawnAIFromClass` "/Game/TriggerForCommander/blueprints/enemy/ThirdPersonBP/Blueprints/enemy1.enemy1_C" null (`SceneComponent.K2_GetComponentLocation` (`self.SpawnPoint`))))
  (bind _asenemy_1 (cast `/Game/TriggerForCommander/blueprints/enemy/ThirdPersonBP/Blueprints/enemy1` _returnvalue))
  (`KismetArrayLibrary.Array_Add` (`self.EnemyList`) _asenemy_1)
  (set `/Game/TriggerForCommander/blueprints/enemy/ThirdPersonBP/Blueprints/enemy1.Spawner` self _asenemy_1))

(fn `UserConstructionScript`)