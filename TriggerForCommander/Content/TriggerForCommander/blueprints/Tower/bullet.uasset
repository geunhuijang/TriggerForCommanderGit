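; Tower bullet actor that homes in on a target enemy in a tower-style game.
; Each tick it moves toward TargetEnemy at Speed and records that enemy's location, continuing toward the last known spot if the target becomes invalid.
; Overlap of its Cube with an enemy1 prints a hit message and destroys the bullet, with no damage applied here.
; A one-second timer from BeginPlay also destroys it.
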(event `self.ReceiveBeginPlay`
  ;[1 1 1] Bullet Destroy Timer
  (`KismetSystemLibrary.Delay` 1.0)
  (`self.K2_DestroyActor`))

(event `self.ReceiveTick`
  (params (DeltaSeconds :type "Float (single-precision)"))
  (bind _targetenemy (`self.TargetEnemy`))
  (bind _returnvalue (`self.K2_GetActorLocation` _targetenemy))
  ;[1 1 1] Bullet Movement
  (`/Engine/EditorBlueprintResources/StandardMacros.IsValid` _targetenemy
    (:`Is Valid`
      (`self.K2_AddActorWorldOffset` (* (`KismetMathLibrary.Normal` (- _returnvalue (`self.K2_GetActorLocation`))) (* DeltaSeconds (`self.Speed`))))
      (`/Engine/EditorBlueprintResources/StandardMacros.IsValid` _targetenemy
        (:`Is Valid`
          (set `self.LastLocation` _returnvalue))))
    (:`Is Not Valid`
      ;[1 1 1] If enemy is not in the scene
      (`self.K2_AddActorWorldOffset` (* (`KismetMathLibrary.Normal` (- (`self.LastLocation`) (`self.K2_GetActorLocation`)) 0.0) (* DeltaSeconds (`self.Speed`)))))))

(event `self.Cube.OnComponentBeginOverlap`
  (params (OverlappedComponent :type "PrimitiveComponent Object Reference") (OtherActor :type "Actor Object Reference") (OtherComp :type "PrimitiveComponent Object Reference") (OtherBodyIndex :type Integer) (bFromSweep :type Boolean) (SweepResult :type "HitResult Structure (by ref)"))
  ;[1 1 1] Enemy Hit
  (cast `/Game/TriggerForCommander/blueprints/enemy/ThirdPersonBP/Blueprints/enemy1` OtherActor)
  (`KismetSystemLibrary.PrintString` "Hit!")
  (`self.K2_DestroyActor`))

(fn `UserConstructionScript`)