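; Tower base actor that serves as a build spot where a tower can be placed.
; BuildTowerOn shows the cursor, clears existing BuildTower widgets, opens a new one linked to this base and the Player, and centers the mouse in the viewport.
; The BuildTower function spawns the Tower class at SpawnPoint's transform and sets HasTower.
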(event `BuildTowerOn`
  (bind _returnvalue (`GameplayStatics.GetPlayerController` 0))
  (bind (_sizex _sizey) (`PlayerController.GetViewportSize` _returnvalue))
  ;[1 1 1] Open Build Tower UI
  (set `PlayerController.bShowMouseCursor` true _returnvalue)
  (bind _foundwidgets (`WidgetBlueprintLibrary.GetAllWidgetsOfClass` "/Game/TriggerForCommander/blueprints/UI/BuildTower.BuildTower_C" false))
  (for _array_element _foundwidgets
    (`Widget.RemoveFromParent` _array_element))
  (bind _returnvalue_2 (`|CreateWidget` "/Game/TriggerForCommander/blueprints/UI/BuildTower.BuildTower_C"))
  (set `/Game/TriggerForCommander/blueprints/UI/BuildTower.TowerBase` self _returnvalue_2)
  (set `/Game/TriggerForCommander/blueprints/UI/BuildTower.Player` (`self.Player`) _returnvalue_2)
  (`UserWidget.AddToViewport` _returnvalue_2 0)
  (`PlayerController.SetMouseLocation` _returnvalue (/ _sizex 2) (/ _sizey 2)))

(fn `BuildTower`
  (`|SpawnActorFromClass` "/Game/TriggerForCommander/blueprints/Tower/Tower.Tower_C" (`SceneComponent.K2_GetComponentToWorld` (`self.SpawnPoint`)) "Undefined" "OverrideRootScale" null null)
  (set `self.HasTower` true))

(fn `UserConstructionScript`)