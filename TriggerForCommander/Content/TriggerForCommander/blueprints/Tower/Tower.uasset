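; Defense tower that auto-fires at the first enemy inside its range sphere, with heat buildup and one-time upgrades.
; Tick aims the body and runs an attack countdown that spawns single-target or AoE bullets.
; Shots add heat that cools over time; overheating blocks fire and swaps materials, while Burst/Normal/Subside states scale attack interval and heat.
; An upgrade widget supports Sniper, Mortar or Machinegun variants, altering range, speed, damage and sometimes mesh.
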(event `self.ReceiveTick`
  (params (DeltaSeconds :type "Float (single-precision)"))
  (bind _body (`self.Body`))
  (bind _attacktimer (`self.AttackTimer`))
  (bind _roll (.roll (`KismetMathLibrary.FindLookAtRotation` (`self.K2_GetActorLocation`) (`self.K2_GetActorLocation` (`|GetArrayItem` (`self.EnemyInSight`))))))
  (bind _yaw (.yaw (`KismetMathLibrary.FindLookAtRotation` (`self.K2_GetActorLocation`) (`self.K2_GetActorLocation` (`|GetArrayItem` (`self.EnemyInSight`))))))
  (`self.OverheatControl`)
  (switch `/Game/TriggerForCommander/blueprints/Tower/TowerUpgrade` (`self.TowerUpgrade`)
    (:`NewEnumerator0`
      (`SceneComponent.K2_SetWorldRotation` _body (`KismetMathLibrary.MakeRotator` _roll 0.0 _yaw) false false :!label _label))
    (:`NewEnumerator1`
      (goto _label))
    (:`NewEnumerator2`
      (`SceneComponent.K2_SetWorldRotation` _body (`KismetMathLibrary.MakeRotator` _roll 0.0 (+ _yaw -90.0)) false false))
    (:`NewEnumerator4`
      (goto _label)))
  (set `self.AttackTimer` (- _attacktimer DeltaSeconds))
  (if (<= _attacktimer 0.0)
    (if (not (== 0 (`KismetArrayLibrary.Array_Length` (`self.EnemyInSight`))))
      (`self.Attack`)
      (set `self.AttackTimer` (* (`self.ASAmp`) (`self.ATK_SPEED`))))))

(event `self.Sphere.OnComponentBeginOverlap`
  (params (OverlappedComponent :type "PrimitiveComponent Object Reference") (OtherActor :type "Actor Object Reference") (OtherComp :type "PrimitiveComponent Object Reference") (OtherBodyIndex :type Integer) (bFromSweep :type Boolean) (SweepResult :type "HitResult Structure (by ref)"))
  ;[1 1 1] Start Attack
  (bind _asenemy_1 (cast `/Game/TriggerForCommander/blueprints/enemy/ThirdPersonBP/Blueprints/enemy1` OtherActor))
  (`KismetArrayLibrary.Array_Add` (`self.EnemyInSight`) _asenemy_1))

(event `self.Sphere.OnComponentEndOverlap`
  (params (OverlappedComponent :type "PrimitiveComponent Object Reference") (OtherActor :type "Actor Object Reference") (OtherComp :type "PrimitiveComponent Object Reference") (OtherBodyIndex :type Integer))
  (bind _enemyinsight (`self.EnemyInSight`))
  ;[1 1 1] Stop Attack
  (bind _asenemy_1 (cast `/Game/TriggerForCommander/blueprints/enemy/ThirdPersonBP/Blueprints/enemy1` OtherActor))
  (`KismetArrayLibrary.Array_RemoveItem` _enemyinsight _asenemy_1)
  (if (== 0 (`KismetArrayLibrary.Array_Length` _enemyinsight))
    _))

(event `UpgradeUIOn`
  (bind _returnvalue (`GameplayStatics.GetPlayerController` 0))
  (bind (_sizex _sizey) (`PlayerController.GetViewportSize` _returnvalue))
  ;[1 1 1] Comment
  (set `PlayerController.bShowMouseCursor` true _returnvalue)
  (bind _foundwidgets (`WidgetBlueprintLibrary.GetAllWidgetsOfClass` "/Game/TriggerForCommander/blueprints/UI/TowerWidget.TowerWidget_C" false))
  (for _array_element _foundwidgets
    (`Widget.RemoveFromParent` _array_element))
  (bind _returnvalue_2 (`|CreateWidget` "/Game/TriggerForCommander/blueprints/UI/TowerWidget.TowerWidget_C"))
  (set `/Game/TriggerForCommander/blueprints/UI/TowerWidget.Tower` self _returnvalue_2)
  (set `/Game/TriggerForCommander/blueprints/UI/TowerWidget.Player` (`self.Player`) _returnvalue_2)
  (`UserWidget.AddToViewport` _returnvalue_2 0)
  (`PlayerController.SetMouseLocation` _returnvalue (/ _sizex 2) (/ _sizey 2)))

(fn `Attack`
  (bind _enemyinsight (`self.EnemyInSight`))
  (bind _atk_damage (`self.ATK_DAMAGE`))
  (bind _returnvalue (`SceneComponent.K2_GetComponentToWorld` (`self.ShootingPoint`)))
  (bind _output (`|GetArrayItem` _enemyinsight))
  (if (`self.OverHeat`)
    (`KismetSystemLibrary.PrintString` "Overheat!!!")
    (elif (!= 0 (`KismetArrayLibrary.Array_Length` _enemyinsight))
      (if (`self.AoeBullet`)
        (bind _returnvalue_2 (`|SpawnActorFromClass` "/Game/TriggerForCommander/blueprints/Tower/AoEBullet.AoEBullet_C" _returnvalue "Undefined" "OverrideRootScale" null null))
        (set `/Game/TriggerForCommander/blueprints/Tower/AoEBullet.Damage` _atk_damage _returnvalue_2)
        (set `/Game/TriggerForCommander/blueprints/Tower/AoEBullet.TargetEnemy` _output _returnvalue_2)
        (else
          (bind _returnvalue_3 (`|SpawnActorFromClass` "/Game/TriggerForCommander/blueprints/Tower/bullet.bullet_C" _returnvalue "Undefined" "OverrideRootScale" null null))
          (set `/Game/TriggerForCommander/blueprints/Tower/bullet.Damage` _atk_damage _returnvalue_3)
          (set `/Game/TriggerForCommander/blueprints/Tower/bullet.TargetEnemy` _output _returnvalue_3)))
      (set `self.Heat` (* (+ (`self.Heat`) (`self.HEAT_PER_ATK`)) (`self.HPAAmp`)))
      (else
        (`KismetSystemLibrary.PrintString` "No Enemy!")))))

(fn `OverheatControl`
  (bind _body (`self.Body`))
  (bind _heat (`self.Heat`))
  (bind _returnvalue (- _heat (* (`GameplayStatics.GetWorldDeltaSeconds`) (`self.COOL_PER_SEC`))))
  (bind _output_get (set `self.OverHeat` (>= _heat (`self.MAX_HEAT`))))
  (switch `/Game/TriggerForCommander/blueprints/Tower/TowerUpgrade` (`self.TowerUpgrade`)
    (:`NewEnumerator0`
      (if _output_get :!label _label
        (`PrimitiveComponent.SetMaterial` _body 0 "/Game/Environment/Materials/M_TD_Arbales_2.M_TD_Arbales_2")
        (else
          (`PrimitiveComponent.SetMaterial` _body 0 "/Game/Environment/Materials/M_TD_Arbales.M_TD_Arbales"))))
    (:`NewEnumerator1`
      (if _output_get
        (`PrimitiveComponent.SetMaterial` _body 0 "/Game/Environment/Materials/M_TD_Cannon_2.M_TD_Cannon_2")
        (else
          (`PrimitiveComponent.SetMaterial` _body 0 "/Game/Environment/Materials/M_TD_Cannon.M_TD_Cannon"))))
    (:`NewEnumerator2`
      (if _output_get
        (`PrimitiveComponent.SetMaterial` _body 0 "/Game/Environment/Materials/M_TD_FlamethrowerTower_2.M_TD_FlamethrowerTower_2")
        (else
          (`PrimitiveComponent.SetMaterial` _body 0 "/Game/Environment/Materials/M_TD_FlamethrowerTower.M_TD_FlamethrowerTower"))))
    (:`NewEnumerator4`
      (goto _label)))
  (if (>= _returnvalue 0.0)
    (set `self.Heat` _returnvalue)
    (else
      (set `self.Heat` 0.0))))

(fn `StateControl`
  (params (State :type "/Game/TriggerForCommander/blueprints/Tower/TowerState Enum" :default "NewEnumerator0"))
  (switch `/Game/TriggerForCommander/blueprints/Tower/TowerState` State
    (:`NewEnumerator0`
      (set `self.TowerState` "NewEnumerator0"))
    (:`NewEnumerator1`
      (set `self.TowerState` "NewEnumerator1"))
    (:`NewEnumerator2`
      (set `self.TowerState` "NewEnumerator2")))
  (switch `/Game/TriggerForCommander/blueprints/Tower/TowerState` (`self.TowerState`)
    (:`NewEnumerator0`
      (set `self.ASAmp` 0.5)
      (set `self.HPAAmp` 1.5)
      (`KismetSystemLibrary.PrintString` "Burst"))
    (:`NewEnumerator1`
      (set `self.ASAmp` 1.0)
      (set `self.HPAAmp` 1.0)
      (`KismetSystemLibrary.PrintString` "Normal"))
    (:`NewEnumerator2`
      (set `self.ASAmp` 2.0)
      (set `self.HPAAmp` 0.0)
      (`KismetSystemLibrary.PrintString` "Subside"))))

(fn `Upgrade`
  (params (UpgradeType :type "/Game/TriggerForCommander/blueprints/Tower/TowerUpgrade Enum" :default "NewEnumerator0"))
  (switch `/Game/TriggerForCommander/blueprints/Tower/TowerUpgrade` (`self.TowerUpgrade`)
    (:`NewEnumerator0`
      (`KismetSystemLibrary.PrintString` "Already Upgraded!" :!label _label))
    (:`NewEnumerator1`
      (goto _label))
    (:`NewEnumerator2`
      (goto _label))
    (:`NewEnumerator4`
      (switch `/Game/TriggerForCommander/blueprints/Tower/TowerUpgrade` UpgradeType
        (:`NewEnumerator0`
          ;[1 1 1] Sniper Upgrade - Range UP, AS DOWN, AD UP
          (`SphereComponent.SetSphereRadius` (`self.Sphere`) (* (`self.ATK_RANGE`) 5.0) true)
          (set `self.ATK_SPEED` (* (`self.ATK_SPEED`) 4.0))
          (set `self.ATK_DAMAGE` (* (`self.ATK_DAMAGE`) 3.0))
          (set `self.TowerUpgrade` "NewEnumerator0"))
        (:`NewEnumerator1`
          ;[1 1 1] Mortar Updrade - Range UP, AS DOWN, AD UP, AoE Damage
          (`SphereComponent.SetSphereRadius` (`self.Sphere`) (* (`self.ATK_RANGE`) 2.0) true)
          (set `self.AoeBullet` true)
          (set `self.ATK_SPEED` (* (`self.ATK_SPEED`) 2.0))
          (set `self.ATK_DAMAGE` (* (`self.ATK_DAMAGE`) 1.5))
          (set `self.TowerUpgrade` "NewEnumerator1")
          (`SkinnedMeshComponent.SetSkinnedAssetAndUpdate` (`self.Body`) "/Game/Environment/Meshes/Cannon_Tower_SkelMesh.Cannon_Tower_SkelMesh" true))
        (:`NewEnumerator2`
          ;[1 1 1] Machinegun Upgrade - Range DOWN, AS UP, AD DOWN
          (`SphereComponent.SetSphereRadius` (`self.Sphere`) (* (`self.ATK_RANGE`) 0.7) true)
          (set `self.ATK_SPEED` (* (`self.ATK_SPEED`) 0.333))
          (set `self.ATK_DAMAGE` (* (`self.ATK_DAMAGE`) 0.75))
          (set `self.TowerUpgrade` "NewEnumerator2")
          (`SkinnedMeshComponent.SetSkinnedAssetAndUpdate` (`self.Body`) "/Game/Environment/Meshes/FlameTower_SkelMesh.FlameTower_SkelMesh" true))))))

(fn `UserConstructionScript`
  (`SphereComponent.SetSphereRadius` (`self.Sphere`) (`self.ATK_RANGE`) true)
  (`self.Upgrade` "NewEnumerator4"))